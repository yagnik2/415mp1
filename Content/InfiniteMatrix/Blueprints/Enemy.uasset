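; Enemy actor that the player must avoid or shoot, with all logic in its event graph.
; Each tick it destroys itself once the player pawn's X location reaches or passes its own.
; An overlap on its Cube component calls ProcessHitEnemy on a BP_Player, while a Fire overlap destroys the enemy and increments the player's PlayerScore.
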(event OnComponentBeginOverlap(Cube)
  (params (OverlappedComponent :type Primitive%20Component%20Object%20Reference) (OtherActor :type Actor%20Object%20Reference) (OtherComp :type Primitive%20Component%20Object%20Reference) (OtherBodyIndex :type Integer) (bFromSweep :type Boolean) (SweepResult :type Hit%20Result%20Structure%20%28by%20ref%29))
  (bind _returnvalue (Utilities|GetClass OtherActor))
  (if (Utilities|ClassIsChildOf _returnvalue "/Game/InfiniteMatrix/Blueprints/BP_Player.BP_Player_C")
    (bind _asbp_player (Utilities|Casting|CastToBP_Player OtherActor))
    (Default|ProcessHitEnemy _asbp_player)
    (elif (Utilities|ClassIsChildOf _returnvalue "/Game/InfiniteMatrix/Blueprints/Fire.Fire_C")
      (Actor|DestroyActor)
      (bind _asbp_player_2 (Utilities|Casting|CastToBP_Player (Game|Player|GetPlayerPawn 0)))
      (Math|Integer|IncrementInt (Variables|/Game/InfiniteMatrix/Blueprints/BP_Player.BP_Player_C|GetPlayerScore _asbp_player_2)))))

(event EventBeginPlay)

(event Collision|EventActorBeginOverlap
  (params (OtherActor :type Actor%20Object%20Reference)))

(event EventTick
  (params (DeltaSeconds :type Float%20%28single-precision%29))
  (if (>= (.x (Transformation|GetActorLocation (Game|Player|GetPlayerPawn 0))) (.x (Transformation|GetActorLocation)))
    (Actor|DestroyActor)))

(fn ConstructionScript)